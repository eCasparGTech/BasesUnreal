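; BP_Killzone is an overlap volume that penalizes a BP_ThirdPersonCharacter for entering it.
; On overlap, a character on its last life triggers a load of DeathMenuMap.
; Otherwise the character teleports to a fixed spawn point set on BeginPlay and loses one of the Lives stored on the character.
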(event EventBeginPlay
  (Variables|Default|SetSpawnPoint "0.000000,0.000000,300.000000"))

(event Collision|EventActorBeginOverlap
  (params (OtherActor :type Actor%20Object%20Reference))
  (bind _asbp_third_person_character (Utilities|Casting|CastToBP_ThirdPersonCharacter OtherActor))
  (if (== (Variables|/Game/ThirdPerson/Blueprints/BP_ThirdPersonCharacter.BP_ThirdPersonCharacter_C|GetLives _asbp_third_person_character) 1)
    (Game|OpenLevel(byName) "DeathMenuMap")
    (else
      (Transformation|Teleport _asbp_third_person_character (Variables|Default|GetSpawnPoint) "0, 0, 0")
      (Variables|/Game/ThirdPerson/Blueprints/BP_ThirdPersonCharacter.BP_ThirdPersonCharacter_C|SetLives _asbp_third_person_character (- (Variables|/Game/ThirdPerson/Blueprints/BP_ThirdPersonCharacter.BP_ThirdPersonCharacter_C|GetLives _asbp_third_person_character) 1)))))

(fn ConstructionScript)