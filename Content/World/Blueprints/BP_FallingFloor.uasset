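; BP_FallingFloor is a floor piece that drops when the third-person player character overlaps it, then resets.
; It stores the static mesh's world location at BeginPlay.
; On overlap it waits briefly, enables physics simulation on the mesh so it falls, then after a few seconds disables physics and teleports it back to the saved location with zeroed rotation.
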(event EventBeginPlay
  (Variables|Default|SetBasePosition (Transformation|GetWorldLocation (Variables|Default|GetStaticMesh))))

(event EventTick
  (params (DeltaSeconds :type Float%20%28single-precision%29)))

(event Collision|EventActorBeginOverlap
  (params (OtherActor :type Actor%20Object%20Reference))
  (bind _staticmesh (Variables|Default|GetStaticMesh))
  (Utilities|Casting|CastToBP_ThirdPersonCharacter OtherActor)
  (Utilities|FlowControl|Delay 0.2)
  (Physics|SetSimulatePhysics (Variables|Default|GetStaticMesh) true)
  (Utilities|FlowControl|Delay 3.0)
  (Physics|SetSimulatePhysics _staticmesh false)
  (Transformation|SetWorldLocation _staticmesh (Variables|Default|GetBasePosition) false true)
  (Transformation|SetWorldRotation _staticmesh "0, 0, 0" false false))

(fn ConstructionScript)